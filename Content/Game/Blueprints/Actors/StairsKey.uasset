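; StairsKey is a trigger actor that toggles a referenced Stairs actor when another actor overlaps it.
; A FlipFlop on begin overlap alternates between calling SlideIn and SlideOut on Stairs.
; A separate MoveIn event, not called within this graph, plays a timeline that offsets the key mesh along Z, scaled by Depth.
; Tick is empty, and the collapse sound and text rotation nodes are disconnected.
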(event Custom|MoveIn
  ;[1 1 1] Move in effect of key
  (bind _newtrack_0 (Timeline|MoveInKey Play)
    (:Update
      (Transformation|SetRelativeLocation (Variables|Default|GetStaticMesh) (Math|Vector|MakeVector 0.0 0.0 (* _newtrack_0 (Variables|Default|Getdepth))) false false))))

(event Collision|EventActorBeginOverlap
  (params (OtherActor :type Actor%20Object%20Reference))
  (bind _stairs (Variables|Default|GetStairs))
  ;[1 1 1] Triggers the stair custom events
  (Utilities|FlowControl|FlipFlop
    (:A
      (Default|Slidein _stairs))
    (:B
      (Default|SlideOut _stairs))))

(event EventTick
  (params (DeltaSeconds :type Float%20%28single-precision%29))
  ;[1 1 1] Text Rotation
)

(fn ConstructionScript)