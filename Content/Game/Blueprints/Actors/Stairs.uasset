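; Stairs actor that slides its stairs in and out through the custom events SlideIn and SlideOut.
; Each event plays its own timeline from the start, scaling the track value by Distance to set the relative location of the Stairs component.
; The EnableY flag selects movement along the Y axis, otherwise along Z.
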(event Custom|SlideIn
  (bind _stairs (Variables|Default|GetStairs))
  ;[1 1 1] Stair slide in custom event in Y- axis
  (bind _newtrack_0 (Timeline|SlideInTimeline PlayFromStart)
    (:Update
      (if (Variables|Default|GetEnableY)
        (Transformation|SetRelativeLocation _stairs (Math|Vector|MakeVector 0.0 (* _newtrack_0 (Variables|Default|GetDistance)) 0.0) false false)
        (else
          (Transformation|SetRelativeLocation _stairs (Math|Vector|MakeVector 0.0 0.0 (* _newtrack_0 (Variables|Default|GetDistance))) false false))))))

(event Custom|SlideOut
  (bind _stairs (Variables|Default|GetStairs))
  ;[1 1 1] Stairs slide out custom event in Y-axis
  (bind _newtrack_0 (Timeline|SlideOutTimeline PlayFromStart)
    (:Update
      (if (Variables|Default|GetEnableY)
        (Transformation|SetRelativeLocation _stairs (Math|Vector|MakeVector 0.0 (* (Variables|Default|GetDistance) _newtrack_0) 0.0) false false)
        (else
          (Transformation|SetRelativeLocation _stairs (Math|Vector|MakeVector 0.0 0.0 (* (Variables|Default|GetDistance) _newtrack_0)) false false))))))

(fn ConstructionScript)